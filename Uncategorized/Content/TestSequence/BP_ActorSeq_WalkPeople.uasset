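; Test Blueprint actor that plays a looping animation, apparently a walking person, until an overlap triggers a different segment of the same Actor Sequence.
; BeginPlay starts the sequence once, and Tick jumps back to the start when the current frame exactly equals the loop-end frame.
; An overlap on the StaticMesh during playback jumps past the loop point to the triggered segment, which is meant to play out and stop.
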(event OnComponentBeginOverlap(StaticMesh)
  (params (OverlappedComponent :type Primitive%20Component%20Object%20Reference) (OtherActor :type Actor%20Object%20Reference) (OtherComp :type Primitive%20Component%20Object%20Reference) (OtherBodyIndex :type Integer) (bFromSweep :type Boolean) (SweepResult :type Hit%20Result%20Structure%20%28by%20ref%29))
  (bind _actorsequence (Variables|Default|GetActorSequence))
  (bind _sequenceplayer (Variables|/Script/ActorSequence.ActorSequenceComponent|GetSequencePlayer _actorsequence))
  ;[1 1 1] 当物体发生触发事件时，理应跳出循环执行触发动画，因此跳转的触发动画位置，继续执行。动画播到结尾处即会停止
  (if (Audio|Components|Audio|IsPlaying _sequenceplayer)
    (Class|MovieSceneSequencePlayer|JumptoSeconds _sequenceplayer 1e+01)))

(event EventBeginPlay
  ;[1 1 1] 游戏运行时开始播放动画，只播一次，循环在Tick里实现
  (Sequencer|Player|Play (Variables|/Script/ActorSequence.ActorSequenceComponent|GetSequencePlayer (Variables|Default|GetActorSequence)) :!class /Script/MovieScene.MovieSceneSequencePlayer))

(event EventTick
  (params (DeltaSeconds :type Float%20%28single-precision%29))
  (bind _actorsequence (Variables|Default|GetActorSequence))
  (bind _sequenceplayer (Variables|/Script/ActorSequence.ActorSequenceComponent|GetSequencePlayer _actorsequence))
  ;[1 1 1] 判断当前动画是否到达循环结束点，是就跳回循环起始点，因为动画并未播到结尾，因此无需再次调用Play，动画还正在Play
  (if (== (Utilities|Struct|BreakFrameNumber (.Frame (Utilities|TimeManagement|BreakQualifiedFrameTime (Sequencer|Player|GetCurrentTime _sequenceplayer)))) 120)
    (Class|MovieSceneSequencePlayer|JumptoSeconds _sequenceplayer 0.0)))

(fn ConstructionScript)