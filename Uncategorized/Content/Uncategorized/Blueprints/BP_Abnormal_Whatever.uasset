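; Clickable "abnormal" object whose static mesh opens a pop-up menu for dealing with it.
; Clicking creates or reuses a UI_PopMenu widget and shows it at the mouse position.
; When the menu already exists, a DoOnce binds its NotifyDealWithAbnormal dispatcher; the creation path skips this binding.
; That notification toggles the mesh's visibility and disables its collision.
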(event OnClicked(StaticMesh)
  (params (TouchedComponent :type Primitive%20Component%20Object%20Reference) (ButtonPressed :type Key%20Structure :default "None"))
  (bind _returnvalue (Game|GetPlayerController 0))
  (bind (_locationx _locationy) (Game|Player|GetMousePosition _returnvalue))
  ;[0 0 0] 在鼠标点击位置添加UMG，并将事件绑定到UMG的按钮点击发送的消息上
  (Utilities|IsValid (Variables|Default|GetPopMenu)
    (:Is%20Valid
      (Utilities|FlowControl|Sequence
        (:then_0
          (Widget|SetVisibility (Variables|Default|GetPopMenu) "Visible" :!label _label)
          (Class|UserWidget|SetPositioninViewport (Variables|Default|GetPopMenu) (Math|Vector2D|MakeVector2D _locationx _locationy) true)
          (UserInterface|Viewport|AddtoViewport (Variables|Default|GetPopMenu) 0))
        (:then_1
          (Utilities|FlowControl|DoOnce false
            (:Completed
              (EventDispatchers|BindEventtoNotifyDealwithAbnormal (stale _output_get) (delegate Custom|Deal%20With%20Abnormal)))))))
    (:Is%20Not%20Valid
      (bind _returnvalue_2 (UserInterface|CreateWidget "/Game/Uncategorized/Blueprints/UMG/UI_PopMenu.UI_PopMenu_C"))
      (bind _output_get (Variables|Default|SetPopMenu _returnvalue_2))
      (goto _label))))

(event Custom|Deal%20With%20Abnormal
  (bind _staticmesh (Variables|Default|GetStaticMesh))
  ;[0 0 0] 在鼠标点击位置添加UMG，并将事件绑定到UMG的按钮点击发送的消息上
  (Rendering|ToggleVisibility _staticmesh false)
  (Collision|SetCollisionEnabled _staticmesh "NoCollision"))

(fn ConstructionScript)